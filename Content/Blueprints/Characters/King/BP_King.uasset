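; BP_King is the king character, who presents answer options to the current subject's dialog.
; On BeginPlay it finds the BP_SubjectSpawner, shows the mouse cursor and disables shadows on its Dialog widget component.
; ShowKingAnswers stores the subject and initializes the WBP_AnswersMain widget with that subject's dialog.
; KingAnswered waits briefly, asks the spawner for a new subject, then hides the stored subject's dialog widget.
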(event Custom|ShowKingAnswers
  (params (Current%20Subject :type BP%20Subject%20Test%20Object%20Reference))
  (Variables|Default|SetCurrentSubject Current%20Subject)
  (Development|PrintString "ShowKingAnswer")
  (bind _aswbp_answers_main (Utilities|Casting|CastToWBP_AnswersMain (UserInterface|GetUserWidgetObject (Variables|Default|GetDialog))))
  (Default|InitializeAnswers _aswbp_answers_main (Variables|/Game/Blueprints/Characters/Subjects/BP_SubjectTest.BP_SubjectTest_C|GetDialog (Variables|Default|GetCurrentSubject))))

(event Custom|KingAnswered
  (Development|PrintString "KingAnswered")
  (Utilities|FlowControl|Delay 2.0)
  (Default|SpawnNewSubject (Variables|Default|GetSpawner))
  (Rendering|SetVisibility (Variables|/Game/Blueprints/Characters/Subjects/BP_SubjectTest.BP_SubjectTest_C|GetDialogWidget (Variables|Default|GetCurrentSubject)) false false))

(event EventBeginPlay
  (bind _returnvalue (Actor|GetActorOfClass "/Game/Blueprints/Spawners/BP_SubjectSpawner.BP_SubjectSpawner_C"))
  (Variables|Default|SetSpawner _returnvalue)
  (Variables|/Script/Engine.PlayerController|SetbShowMouseCursor (Game|GetPlayerController 0) true)
  (Rendering|SetCastShadow (Variables|Default|GetDialog) false))

(event Collision|EventActorBeginOverlap
  (params (OtherActor :type Actor%20Object%20Reference)))

(event EventTick
  (params (DeltaSeconds :type Float%20%28single-precision%29)))

(fn ConstructionScript)