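; Stanczyk character Blueprint that displays the character's answers in a world-placed Dialog widget component.
; StanczykAnswer reveals the widget and passes the answer to WBP_Dialog's StartAnswer with a fixed subject ID identifying the speaker.
; Every tick, the widget copies the player's view rotation with a fixed pitch offset, and its shadow is disabled on BeginPlay.
; StanczykAnswered is an empty event.
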(event Custom|StanczykAnswer
  (params (Answer :type String))
  (Rendering|SetVisibility (Variables|Default|GetDialog) true false)
  (bind _aswbp_dialog (Utilities|Casting|CastToWBP_Dialog (UserInterface|GetUserWidgetObject (Variables|Default|GetDialog))))
  (Default|StartAnswer _aswbp_dialog Answer 0 2))

(event Custom|StanczykAnswered)

(event EventBeginPlay
  (Rendering|SetCastShadow (Variables|Default|GetDialog) false))

(event Collision|EventActorBeginOverlap
  (params (OtherActor :type Actor%20Object%20Reference)))

(event EventTick
  (params (DeltaSeconds :type Float%20%28single-precision%29))
  (bind _returnvalue (Game|Player|GetPlayerPawn 0))
  (bind _outrotation (Actor|GetActorEyesViewPoint _returnvalue))
  (Transformation|SetWorldRotation (Variables|Default|GetDialog) (Math|Rotator|MakeRotator (.roll _outrotation) (+ (.pitch _outrotation) 3e+01) (.yaw _outrotation)) false false))

(fn ConstructionScript)