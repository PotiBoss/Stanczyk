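; BP_SubjectTest is a subject character that queues at spawner-defined spots and brings a question to the King.
; On BeginPlay it caches the spawner and King and picks a random dialog index.
; MoveInQueue advances its queue spot through simple AI movement, while SubjectQuestion shows the dialog widget and starts that dialog with the King and itself.
; Tick aligns the widget to the player's view rotation with a pitch offset.
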(event Custom|MoveInQueue
  (bind _result (Math|Integer|IncrementInt (Variables|Default|GetQueueSpot))
    (:%20%20
      (AI|Navigation|SimpleMovetoLocation (Pawn|GetController) (+ (Utilities|Array|Get(acopy) (Variables|/Game/Blueprints/Spawners/BP_SubjectSpawner.BP_SubjectSpawner_C|GetSpots (Variables|Default|GetSpawner)) _result) (Transformation|GetActorLocation (Variables|Default|GetSpawner)))))))

(event Custom|SubjectQuestion
  (bind _dialogwidget (Variables|Default|GetDialogWidget))
  (Rendering|SetVisibility _dialogwidget true false)
  (bind _aswbp_dialog (Utilities|Casting|CastToWBP_Dialog (UserInterface|GetUserWidgetObject _dialogwidget)))
  (Default|StartDialog _aswbp_dialog (Variables|Default|GetDialogIndex) (Variables|Default|GetKing) 0 self))

(event EventBeginPlay
  (bind _returnvalue (Actor|GetActorOfClass "/Game/Blueprints/Spawners/BP_SubjectSpawner.BP_SubjectSpawner_C"))
  (Variables|Default|SetSpawner _returnvalue)
  (bind _returnvalue_2 (Actor|GetActorOfClass "/Game/Blueprints/Characters/King/BP_King.BP_King_C"))
  (Variables|Default|SetKing _returnvalue_2)
  (Rendering|SetCastShadow (Variables|Default|GetDialogWidget) false)
  (Variables|Default|SetDialogIndex (Math|Random|RandomIntegerinRange 1 30)))

(event Collision|EventActorBeginOverlap
  (params (OtherActor :type Actor%20Object%20Reference)))

(event EventTick
  (params (DeltaSeconds :type Float%20%28single-precision%29))
  (bind _returnvalue (Game|Player|GetPlayerPawn 0))
  (bind _outrotation (Actor|GetActorEyesViewPoint _returnvalue))
  (Transformation|SetWorldRotation (Variables|Default|GetDialogWidget) (Math|Rotator|MakeRotator (.roll _outrotation) (+ (.pitch _outrotation) 3e+01) (.yaw _outrotation)) false false))

(fn ConstructionScript)