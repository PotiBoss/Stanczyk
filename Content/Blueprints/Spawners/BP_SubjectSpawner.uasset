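; Spawner actor that feeds a queue of randomly chosen subjects into the level and triggers their questions.
; On BeginPlay it spawns three subjects at two-second intervals at its own transform, picking each class at random from a list.
; After each spawn it records the subject and tells every spawned subject to advance in the queue.
; Subjects overlapping the Talk component are prompted to ask their question.
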(event OnComponentBeginOverlap(Talk)
  (params (OverlappedComponent :type Primitive%20Component%20Object%20Reference) (OtherActor :type Actor%20Object%20Reference) (OtherComp :type Primitive%20Component%20Object%20Reference) (OtherBodyIndex :type Integer) (bFromSweep :type Boolean) (SweepResult :type Hit%20Result%20Structure%20%28by%20ref%29))
  (bind _asbp_subject_test (Utilities|Casting|CastToBP_SubjectTest OtherActor))
  (Default|SubjectQuestion _asbp_subject_test))

(event Custom|SpawnNewSubject
  (bind _returnvalue (Game|SpawnActorfromClass (.OutItem (Utilities|Array|Random (Variables|Default|GetSubjectClasses))) (Transformation|GetActorTransform) "Undefined" 0 0))
  (Utilities|Array|Add (Variables|Default|GetSpawnedSubjects) _returnvalue)
  (CallFunction|MoveAllSubjects))

(event Custom|MoveAllSubjects
  (for _array_element (Variables|Default|GetSpawnedSubjects)
    (Default|MoveinQueue _array_element)))

(event EventBeginPlay
  (Utilities|FlowControl|Delay 2.0)
  (CallFunction|SpawnNewSubject)
  (Utilities|FlowControl|Delay 2.0)
  (CallFunction|SpawnNewSubject)
  (Utilities|FlowControl|Delay 2.0)
  (CallFunction|SpawnNewSubject))

(event Collision|EventActorBeginOverlap
  (params (OtherActor :type Actor%20Object%20Reference)))

(event EventTick
  (params (DeltaSeconds :type Float%20%28single-precision%29)))

(fn ConstructionScript)